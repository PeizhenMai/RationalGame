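; BP_Obstacle is an obstacle actor that makes zombies jump when they reach it.
; It has four collision components, each with its own begin-overlap event.
; Each event casts the overlapping actor to BP_Zombie and calls Jump on it, ignoring any other actor.
; The construction script is empty.
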(event OnComponentBeginOverlap(Obstacle_Collison4)
  (params (OverlappedComponent :type Primitive%20Component%20Object%20Reference) (OtherActor :type Actor%20Object%20Reference) (OtherComp :type Primitive%20Component%20Object%20Reference) (OtherBodyIndex :type Integer) (bFromSweep :type Boolean) (SweepResult :type Hit%20Result%20Structure%20%28by%20ref%29))
  (bind _asbp_zombie (Utilities|Casting|CastToBP_Zombie OtherActor))
  (Character|Jump _asbp_zombie))

(event OnComponentBeginOverlap(Obstacle_Collison3)
  (params (OverlappedComponent :type Primitive%20Component%20Object%20Reference) (OtherActor :type Actor%20Object%20Reference) (OtherComp :type Primitive%20Component%20Object%20Reference) (OtherBodyIndex :type Integer) (bFromSweep :type Boolean) (SweepResult :type Hit%20Result%20Structure%20%28by%20ref%29))
  (bind _asbp_zombie (Utilities|Casting|CastToBP_Zombie OtherActor))
  (Character|Jump _asbp_zombie))

(event OnComponentBeginOverlap(Obstacle_Collison1)
  (params (OverlappedComponent :type Primitive%20Component%20Object%20Reference) (OtherActor :type Actor%20Object%20Reference) (OtherComp :type Primitive%20Component%20Object%20Reference) (OtherBodyIndex :type Integer) (bFromSweep :type Boolean) (SweepResult :type Hit%20Result%20Structure%20%28by%20ref%29))
  (bind _asbp_zombie (Utilities|Casting|CastToBP_Zombie OtherActor))
  (Character|Jump _asbp_zombie))

(event OnComponentBeginOverlap(Obstacle_Collison2)
  (params (OverlappedComponent :type Primitive%20Component%20Object%20Reference) (OtherActor :type Actor%20Object%20Reference) (OtherComp :type Primitive%20Component%20Object%20Reference) (OtherBodyIndex :type Integer) (bFromSweep :type Boolean) (SweepResult :type Hit%20Result%20Structure%20%28by%20ref%29))
  (bind _asbp_zombie (Utilities|Casting|CastToBP_Zombie OtherActor))
  (Character|Jump _asbp_zombie))

(fn ConstructionScript)