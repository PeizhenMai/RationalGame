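; BP_Zombie is an enemy character that chases the player's top-down character when it comes within sight range.
; BeginPlay caches the player and spawns a default controller.
; Every tick it turns to face the player and, inside the Sight distance, moves straight toward them with AddMovementInput rather than pathfinding.
; The construction script, gated by a DungeonGameInstance cast, loads walk speed, sight and health from the Level1 row of DT_Zombie.
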(event EventBeginPlay
  (bind _asbp_top_down_character (Utilities|Casting|CastToBP_TopDownCharacter (Game|GetPlayerCharacter 0)))
  (Variables|Default|SetCharacter _asbp_top_down_character)
  (Pawn|SpawnDefaultController))

(event EventTick
  (params (DeltaSeconds :type Float%20%28single-precision%29))
  (Utilities|IsValid (Variables|Default|GetCharacter)
    (:Is%20Valid
      (bind _output_get (Variables|Default|SetZombieLocation (Transformation|GetActorLocation)))
      (bind _output_get_2 (Variables|Default|SetCharacterLocation (Transformation|GetActorLocation (Variables|Default|GetCharacter))))
      (Variables|Default|SetDistance (Math|Vector|VectorLength (- (Variables|Default|GetCharacterLocation) (Variables|Default|GetZombieLocation))))
      (Transformation|SetActorRotation (Math|Rotator|FindLookatRotation _output_get _output_get_2))
      (if (<= (Variables|Default|GetDistance) (Variables|Default|GetSight))
        (Development|PrintString "Detected Player")
        (Pawn|Input|AddMovementInput (Math|Vector|Normalize (- (Variables|Default|GetCharacterLocation) (Variables|Default|GetZombieLocation))) 1.0 false)))))

(fn ConstructionScript
  (Utilities|Casting|CastToDungeonGameInstance (Game|GetGameInstance))
  (bind _returnvalue (Utilities|GetDataTableRow "/Game/DataTable/DT_Zombie.DT_Zombie" "Level1")
    (:then
      (Variables|/Script/Engine.CharacterMovementComponent|SetMaxWalkSpeed (Variables|Character|GetCharacterMovement) (.walkspeed _returnvalue))
      (Variables|Default|SetSight (.detecteddistance _returnvalue))
      (Variables|Default|SetHealth (.zombiehealth _returnvalue)))))