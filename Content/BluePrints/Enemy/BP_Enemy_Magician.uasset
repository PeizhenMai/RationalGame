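; Magician enemy that chases the player within sight range, takes hits shown on its widget, and awards random gold on death.
; Construction loads its stats from DT_Magician by the game instance's level name.
; Tick grows an array as a "temper" meter while the player is visible, draining it otherwise; at full it clears and sets Attacking.
; AttackCharacter, not called here, spawns an overhead meteor launched at the player.
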(event EventBeginPlay
  (Utilities|FlowControl|Sequence
    (:then_0
      (bind _asbp_top_down_character (Utilities|Casting|CastToBP_TopDownCharacter (Game|GetPlayerCharacter 0)))
      (Variables|Default|SetAs%20BP%20Top%20Down%20Character _asbp_top_down_character))
    (:then_1
      (bind _aswb_magician (Utilities|Casting|CastToWB_Magician (UserInterface|GetWidget (Variables|Default|GetWidget))))
      (Variables|/Game/Widget/WB_Magician.WB_Magician_C|SetPercentage _aswb_magician (Variables|Default|GetHealthPercentage))
      (Variables|/Game/Widget/WB_Magician.WB_Magician_C|SetTemper%20Percentage _aswb_magician (Variables|Default|GetTemperPercentage)))
    (:then_2
      (Pawn|SpawnDefaultController))))

(event EventCharacterAttack
  ;[1 1 1] Being attacked
  (bind _output_get (Variables|Default|SetCurrentHealth (- (Variables|Default|GetCurrentHealth) (Variables|/Game/PlayerCharacter/Blueprints/BP_TopDownCharacter.BP_TopDownCharacter_C|GetCurrentAttackDamage (Variables|Default|GetAs%20BP%20Top%20Down%20Character)))))
  (bind _aswb_magician (Utilities|Casting|CastToWB_Magician (UserInterface|GetWidget (Variables|Default|GetWidget))))
  (Variables|/Game/Widget/WB_Magician.WB_Magician_C|SetPercentage _aswb_magician (/ _output_get (Variables|Default|GetMaxHealth)))
  (Variables|/Game/PlayerCharacter/Blueprints/BP_TopDownCharacter.BP_TopDownCharacter_C|SetbCharacterCanAttack (Variables|Default|GetAs%20BP%20Top%20Down%20Character) false))

(event EventTick
  (params (DeltaSeconds :type Float%20%28single-precision%29))
  (Utilities|IsValid (Variables|Default|GetAs%20BP%20Top%20Down%20Character)
    (:Is%20Valid
      (Utilities|FlowControl|Sequence
        (:then_0
          ;[1 1 1] Percentage
          (Variables|Default|SetTemperPercentage (/ (Math|Conversions|ToFloat(Integer) (Utilities|Array|Length (Variables|Default|GetTemper%20Array))) 3e+02)))
        (:then_1
          (if (not (Variables|Default|GetbIsDead))
            ;[1 1 1] Go to character
            (if (Variables|Default|GetbCanSee)
              (Transformation|SetActorRotation (Math|Rotator|FindLookatRotation (Variables|Default|GetMagicianLocation) (Variables|Default|GetCharacterLocation)))
              (Pawn|Input|AddMovementInput (Math|Vector|Normalize (- (Variables|Default|GetCharacterLocation) (Variables|Default|GetMagicianLocation))) 1.0 false))))
        (:then_2
          ;[1 1 1] Attack Character
          (bind _aswb_magician (Utilities|Casting|CastToWB_Magician (UserInterface|GetWidget (Variables|Default|GetWidget))))
          (Variables|/Game/Widget/WB_Magician.WB_Magician_C|SetTemper%20Percentage _aswb_magician (Variables|Default|GetTemperPercentage))
          (if (== (Utilities|Array|Length (Variables|Default|GetTemper%20Array)) 300)
            (Utilities|FlowControl|Sequence
              (:then_0
                (Utilities|Array|Clear (Variables|Default|GetTemper%20Array)))
              (:then_1
                (Variables|Default|SetbAttacking true)))))
        (:then_3
          ;[1 1 1] detect distance
          (Variables|Default|SetMagicianLocation (Transformation|GetActorLocation))
          (Variables|Default|SetCharacterLocation (Transformation|GetActorLocation (Variables|Default|GetAs%20BP%20Top%20Down%20Character)))
          (if (<= (Math|Vector|VectorLengthXY (- (Variables|Default|GetCharacterLocation) (Variables|Default|GetMagicianLocation))) (Variables|Default|GetSIght))
            (Variables|Default|SetbCanSee true)
            (CallFunction|GetTemper)
            (else
              (Variables|Default|SetbCanSee false)
              (for (_ _array_index) (Variables|Default|GetTemper%20Array)
                (Utilities|FlowControl|Delay 0.05)
                (Utilities|Array|RemoveIndex (Variables|Default|GetTemper%20Array) _array_index)))))
        (:then_4
          ;[1 1 1] Dead Condition
          (if (<= (Variables|Default|GetCurrentHealth) 0.0)
            (Variables|Default|SetbIsDead true)
            (Utilities|FlowControl|DoOnce false
              (:Completed
                (CallFunction|MagicianDead)
                (Utilities|FlowControl|Delay 5.0)
                (Actor|DestroyActor)))))
        (:then_5
          ;[1 1 1] Current Speed
          (Variables|Default|SetCurrentSpeed (Math|Vector|VectorLengthXY (Variables|/Script/Engine.MovementComponent|GetVelocity (Variables|Character|GetCharacterMovement)))))))))

(fn ConstructionScript
  (|CallParentFunction)
  (bind _asdungeon_game_instance (Utilities|Casting|CastToDungeonGameInstance (Game|GetGameInstance)))
  (bind _returnvalue (Utilities|GetDataTableRow "/Game/DataTable/DT_Magician.DT_Magician" (Variables|/Game/DungeonGameInstance.DungeonGameInstance_C|GetLevelName _asdungeon_game_instance))
    (:then
      (Variables|/Script/Engine.CharacterMovementComponent|SetMaxWalkSpeed (Variables|Character|GetCharacterMovement) (.maxwalkspeed _returnvalue))
      (bind _output_get (Variables|Default|SetMaxHealth (.magicianhealth _returnvalue)))
      (Variables|Default|SetCurrentHealth _output_get)
      (Variables|Default|SetSight (.sight _returnvalue))
      (Variables|Default|SetAttackDamage (.magicianattack _returnvalue))
      (Variables|Default|SetAttackSpeed (.magicianattackspeed _returnvalue))
      (Variables|Default|SetDropGold (Math|Random|RandomIntegerinRange (.mingold _returnvalue) (.maxgold _returnvalue))))))

(fn MagicianDead
  (Rendering|SetVisibility (Variables|Default|GetWidget) false false)
  (Collision|SetCollisionEnabled (Variables|Default|GetCapsuleComponent) "NoCollision")
  (bind _asdungeon_game_instance (Utilities|Casting|CastToDungeonGameInstance (Game|GetGameInstance)))
  (Variables|/Game/DungeonGameInstance.DungeonGameInstance_C|SetGold _asdungeon_game_instance (+ (Variables|/Game/DungeonGameInstance.DungeonGameInstance_C|GetGold _asdungeon_game_instance) (Variables|Default|GetDropGold))))

(fn GetTemper
  (bind _output_get (LocalVariables|SetCurrentTime (Utilities|Time|GetGameTimeinSeconds)))
  (Utilities|Array|Add (Variables|Default|GetTemper%20Array) _output_get))

(fn AttackCharacter
  (bind _returnvalue (Transformation|GetActorLocation))
  (bind _output_get (LocalVariables|SetMeteorLocation (Math|Vector|MakeVector (.x _returnvalue) (.y _returnvalue) (+ (.z _returnvalue) 1e+03))))
  (bind _returnvalue_2 (Game|SpawnActorfromClass "/Game/BluePrints/BP_Meteor.BP_Meteor_C" (Math|Transform|MakeTransform _output_get "0, 0, 0" "1.000000,1.000000,1.000000") "Undefined" "MultiplyWithRoot" 0 0))
  (bind _output_get_2 (LocalVariables|SetTargetLocation (Transformation|GetActorLocation (Variables|Default|GetAs%20BP%20Top%20Down%20Character))))
  (Class|BPIHitcharacter|MeteorImpulse(Message) _returnvalue_2 (- _output_get_2 (LocalVariables|GetMeteorLocation)) (Variables|Default|GetAttackDamage)))