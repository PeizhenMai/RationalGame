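; Zombie enemy for the dungeon game that detects the player, rewarding gold and experience on death.
; Construction loads stats from DT_Zombie by the game instance's level name and rolls the rewards.
; Tick latches sight by XY distance, then drives facing and direct movement input without pathfinding.
; Box overlaps toggle an attacking flag; CharacterAttack applies damage to health and widget, with death leading to delayed destruction.
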(event OnComponentBeginOverlap(Box)
  (params (OverlappedComponent :type Primitive%20Component%20Object%20Reference) (OtherActor :type Actor%20Object%20Reference) (OtherComp :type Primitive%20Component%20Object%20Reference) (OtherBodyIndex :type Integer) (bFromSweep :type Boolean) (SweepResult :type Hit%20Result%20Structure%20%28by%20ref%29))
  ;[1 1 1] Attack Character
  (if (== OtherActor (Variables|Default|GetCharacterRef))
    (Variables|Default|SetbAttacking true)))

(event OnComponentEndOverlap(Box)
  (params (OverlappedComponent :type Primitive%20Component%20Object%20Reference) (OtherActor :type Actor%20Object%20Reference) (OtherComp :type Primitive%20Component%20Object%20Reference) (OtherBodyIndex :type Integer))
  ;[1 1 1] Attack Character
  (if (== OtherActor (Variables|Default|GetCharacterRef))
    (Variables|Default|SetbAttacking false)))

(event EventBeginPlay
  (Utilities|FlowControl|Sequence
    (:then_0
      (bind _aswb_zombie (Utilities|Casting|CastToWB_Zombie (UserInterface|GetWidget (Variables|Default|GetWidget))))
      (Variables|/Game/Widget/WB_Zombie.WB_Zombie_C|SetPercentage _aswb_zombie (Variables|Default|GetHealthPercentage)))
    (:then_1
      (Pawn|SpawnDefaultController))
    (:then_2
      (bind _asbp_top_down_character (Utilities|Casting|CastToBP_TopDownCharacter (Game|GetPlayerCharacter 0)))
      (Variables|Default|SetCharacterRef _asbp_top_down_character))))

(event EventTick
  (params (DeltaSeconds :type Float%20%28single-precision%29))
  (Utilities|IsValid (Variables|Default|GetCharacterRef)
    (:Is%20Valid
      (Utilities|FlowControl|Sequence
        (:then_0
          (if (not (Variables|Default|GetbIsDead))
            ;[1 1 1] Walk to Character
            (if (Variables|Default|GetbCanSee)
              (Transformation|SetActorRotation (Math|Rotator|FindLookatRotation (Variables|Default|GetZombieLocation) (Variables|Default|GetCharacterLocation)))
              (Pawn|Input|AddMovementInput (Math|Vector|Normalize (- (Variables|Default|GetZombieLocation) (Variables|Default|GetCharacterLocation))) 1.0 false))))
        (:then_1
          ;[1 1 1] detect distance
          (Variables|Default|SetZombieLocation (Transformation|GetActorLocation))
          (Variables|Default|SetCharacterLocation (Transformation|GetActorLocation (Variables|Default|GetCharacterRef)))
          (if (<= (Math|Vector|VectorLengthXY (- (Variables|Default|GetCharacterLocation) (Variables|Default|GetZombieLocation))) (Variables|Default|GetSight))
            (Variables|Default|SetbCanSee true)))
        (:then_2
          ;[1 1 1] Zombie Dead
          (if (<= (Variables|Default|GetCurrentHealth) 0.0)
            (Variables|Default|SetbIsDead true)
            (Utilities|FlowControl|DoOnce false
              (:Completed
                (CallFunction|ZombieDead)
                (Utilities|FlowControl|Delay 3.0)
                (Actor|DestroyActor)))))))))

(event EventCharacterAttack
  ;[1 1 1] Being Attacked
  (bind _output_get (Variables|Default|SetCurrentHealth (- (Variables|Default|GetCurrentHealth) (Variables|/Game/PlayerCharacter/Blueprints/BP_TopDownCharacter.BP_TopDownCharacter_C|GetCurrentAttackDamage (Variables|Default|GetCharacterRef)))))
  (bind _aswb_zombie (Utilities|Casting|CastToWB_Zombie (UserInterface|GetWidget (Variables|Default|GetWidget))))
  (Variables|/Game/Widget/WB_Zombie.WB_Zombie_C|SetPercentage _aswb_zombie (/ _output_get (Variables|Default|GetMaxHealth)))
  (Variables|/Game/PlayerCharacter/Blueprints/BP_TopDownCharacter.BP_TopDownCharacter_C|SetbCharacterCanAttack (Variables|Default|GetCharacterRef) false))

(event Collision|EventActorBeginOverlap
  (params (OtherActor :type Actor%20Object%20Reference)))

(fn ConstructionScript
  (|CallParentFunction)
  (bind _asdungeon_game_instance (Utilities|Casting|CastToDungeonGameInstance (Game|GetGameInstance)))
  (bind _returnvalue (Utilities|GetDataTableRow "/Game/DataTable/DT_Zombie.DT_Zombie" (Variables|/Game/DungeonGameInstance.DungeonGameInstance_C|GetLevelName _asdungeon_game_instance))
    (:then
      (Variables|/Script/Engine.CharacterMovementComponent|SetMaxWalkSpeed (Variables|Character|GetCharacterMovement) (.maxwalkspeed _returnvalue))
      (bind _output_get (Variables|Default|SetMaxHealth (.zombiehealth _returnvalue)))
      (Variables|Default|SetCurrentHealth _output_get)
      (Variables|Default|SetSight (.zombiesight _returnvalue))
      (Variables|Default|SetAttackDamage (.zombieattack _returnvalue))
      (Variables|Default|SetDropGold (Math|Random|RandomIntegerinRange (.mingold _returnvalue) (.maxgold _returnvalue)))
      (Variables|Default|SetExp (Math|Random|RandomFloatinRange (.minexp _returnvalue) (.maxexp _returnvalue))))))

(fn ZombieDead
  (Rendering|SetVisibility (Variables|Default|GetWidget) false false)
  (Collision|SetCollisionEnabled (Variables|Default|GetCapsuleComponent) "NoCollision")
  (bind _asdungeon_game_instance (Utilities|Casting|CastToDungeonGameInstance (Game|GetGameInstance)))
  (Variables|/Game/DungeonGameInstance.DungeonGameInstance_C|SetGold _asdungeon_game_instance (+ (Variables|/Game/DungeonGameInstance.DungeonGameInstance_C|GetGold _asdungeon_game_instance) (Variables|Default|GetDropGold)))
  (Variables|/Game/DungeonGameInstance.DungeonGameInstance_C|SetCharacterExp _asdungeon_game_instance (+ (Variables|/Game/DungeonGameInstance.DungeonGameInstance_C|GetCharacterExp _asdungeon_game_instance) (Variables|Default|GetExp))))