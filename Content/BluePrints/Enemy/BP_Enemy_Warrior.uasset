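; Warrior enemy for a dungeon game that chases the player within sight range and awards gold on death.
; Construction script loads stats and random gold drop from DT_Warrior, keyed by the game instance's level name.
; Tick updates health percentage, checks XY distance to steer directly toward the player without pathfinding, and triggers one-time death and delayed destruction.
; CharacterAttack applies the player's damage, updates the health widget and clears the player's can-attack flag.
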(event Custom|Jump%20To%20Character
  (Development|PrintString "Hello"))

(event EventBeginPlay
  (Utilities|FlowControl|Sequence
    (:then_0
      (bind _asbp_top_down_character (Utilities|Casting|CastToBP_TopDownCharacter (Game|GetPlayerCharacter 0)))
      (Variables|Default|SetAs%20BP%20Top%20Down%20Character _asbp_top_down_character))
    (:then_1
      (Pawn|SpawnDefaultController))
    (:then_2
      (bind _aswb_warrior (Utilities|Casting|CastToWB_Warrior (UserInterface|GetWidget (Variables|Default|GetWidget))))
      (Variables|/Game/Widget/WB_Warrior.WB_Warrior_C|SetPercentage _aswb_warrior (Variables|Default|GetHealthPercentage)))))

(event EventCharacterAttack
  ;[1 1 1] Being Attack
  (Variables|Default|SetCurrrentHealth (- (Variables|Default|GetCurrrentHealth) (Variables|/Game/PlayerCharacter/Blueprints/BP_TopDownCharacter.BP_TopDownCharacter_C|GetCurrentAttackDamage (Variables|Default|GetAs%20BP%20Top%20Down%20Character))))
  (bind _aswb_warrior (Utilities|Casting|CastToWB_Warrior (UserInterface|GetWidget (Variables|Default|GetWidget))))
  (Variables|/Game/Widget/WB_Warrior.WB_Warrior_C|SetPercentage _aswb_warrior (Variables|Default|GetHealthPercentage))
  (Variables|/Game/PlayerCharacter/Blueprints/BP_TopDownCharacter.BP_TopDownCharacter_C|SetbCharacterCanAttack (Variables|Default|GetAs%20BP%20Top%20Down%20Character) false))

(event EventTick
  (params (DeltaSeconds :type Float%20%28single-precision%29))
  (Utilities|IsValid (Variables|Default|GetAs%20BP%20Top%20Down%20Character)
    (:Is%20Valid
      (Utilities|FlowControl|Sequence
        (:then_0
          ;[1 1 1] HP Percentage
          (Variables|Default|SetHealthPercentage (/ (Variables|Default|GetCurrrentHealth) (Variables|Default|GetMaxHealth))))
        (:then_1
          (if (not (Variables|Default|GetbIsDead))
            (if (Variables|Default|GetbCanSee)
              ;[1 1 1] Go to Character
              (Transformation|SetActorRotation (Math|Rotator|FindLookatRotation (Variables|Default|GetWarriorLocation) (Variables|Default|GetCharacterLocation)))
              (Pawn|Input|AddMovementInput (Math|Vector|Normalize (- (Variables|Default|GetCharacterLocation) (Variables|Default|GetWarriorLocation))) 1.0 false))))
        (:then_2
          ;[1 1 1] Detect Distrance
          (Variables|Default|SetWarriorLocation (Transformation|GetActorLocation))
          (Variables|Default|SetCharacterLocation (Transformation|GetActorLocation (Variables|Default|GetAs%20BP%20Top%20Down%20Character)))
          (if (<= (Math|Vector|VectorLengthXY (- (Variables|Default|GetCharacterLocation) (Variables|Default|GetWarriorLocation))) (Variables|Default|GetSIght))
            (Variables|Default|SetbCanSee true)
            (Variables|Default|SetbHasSeen true)
            (else
              (Variables|Default|SetbCanSee false)
              (if (Variables|Default|GetbHasSeen)
                _))))
        (:then_3
          ;[1 1 1] Dead Condition
          (if (<= (Variables|Default|GetCurrrentHealth) 0.0)
            (Variables|Default|SetbIsDead true)
            (Utilities|FlowControl|DoOnce false
              (:Completed
                (CallFunction|WarriorDead)
                (Utilities|FlowControl|Delay 5.0)
                (Actor|DestroyActor)))))))))

(fn ConstructionScript
  (|CallParentFunction)
  (bind _asdungeon_game_instance (Utilities|Casting|CastToDungeonGameInstance (Game|GetGameInstance)))
  (bind _returnvalue (Utilities|GetDataTableRow "/Game/DataTable/DT_Warrior.DT_Warrior" (Variables|/Game/DungeonGameInstance.DungeonGameInstance_C|GetLevelName _asdungeon_game_instance))
    (:then
      (bind _output_get (Variables|Default|SetMaxHealth (.warriorhealth _returnvalue)))
      (Variables|Default|SetCurrrentHealth _output_get)
      (Variables|/Script/Engine.CharacterMovementComponent|SetMaxWalkSpeed (Variables|Character|GetCharacterMovement) (.maxwalkspeed _returnvalue))
      (Variables|Default|SetDropGold (Math|Random|RandomIntegerinRange (.mingold _returnvalue) (.maxgold _returnvalue)))
      (Variables|Default|SetSight (.sight _returnvalue))
      (Variables|Default|SetAttackDamage (.warriorattack _returnvalue))
      (Variables|Default|SetAttackSpeed (.warriorattackspeed _returnvalue)))))

(fn WarriorDead
  (Rendering|SetVisibility (Variables|Default|GetWidget) false false)
  (Collision|SetCollisionEnabled (Variables|Default|GetCapsuleComponent) "NoCollision")
  (bind _asdungeon_game_instance (Utilities|Casting|CastToDungeonGameInstance (Game|GetGameInstance)))
  (Variables|/Game/DungeonGameInstance.DungeonGameInstance_C|SetGold _asdungeon_game_instance (+ (Variables|/Game/DungeonGameInstance.DungeonGameInstance_C|GetGold _asdungeon_game_instance) (Variables|Default|GetDropGold))))