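; BP_Meteor is a physics-driven meteor projectile that damages the player's BP_TopDownCharacter on contact.
; MeteorImpulse launches it by applying a scaled impulse to its Sphere.
; Sphere1 overlaps send a MagicianHit message with damage to the cached player, then destroy the meteor shortly after.
; Overlaps with any other actor destroy it after a longer delay; its own MagicianHit and ZombieHit functions are empty.
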(event OnComponentBeginOverlap(Sphere1)
  (params (OverlappedComponent :type Primitive%20Component%20Object%20Reference) (OtherActor :type Actor%20Object%20Reference) (OtherComp :type Primitive%20Component%20Object%20Reference) (OtherBodyIndex :type Integer) (bFromSweep :type Boolean) (SweepResult :type Hit%20Result%20Structure%20%28by%20ref%29))
  (if (== OtherActor (Variables|Default|GetAs%20BP%20Top%20Down%20Character))
    (Class|BPIHitcharacter|MagicianHit(Message) (Variables|Default|GetAs%20BP%20Top%20Down%20Character) (stale EventMeteorImpulse Damage))
    (Utilities|FlowControl|Delay 0.2)
    (Actor|DestroyActor)
    (else
      (Utilities|FlowControl|Delay 2.0)
      (Actor|DestroyActor))))

(event EventBeginPlay
  (bind _asbp_top_down_character (Utilities|Casting|CastToBP_TopDownCharacter (Game|GetPlayerCharacter 0)))
  (Variables|Default|SetAs%20BP%20Top%20Down%20Character _asbp_top_down_character))

(event EventMeteorImpulse
  (params (ImpulseVector :type Vector :default "0, 0, 0") (Damage :type Float%20%28double-precision%29))
  (Physics|AddImpulse (Variables|Default|GetSphere) (* ImpulseVector "30.000000,30.000000,30.000000") "None" false))

(fn ConstructionScript)

(fn MagicianHit
  (params (Damage :type Float%20%28double-precision%29)))

(fn ZombieHit
  (params (Damage :type Float%20%28double-precision%29))
  (return))