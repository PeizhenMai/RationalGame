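; Upgrade room, derived from a parent room class, that offers the player HP and magic restoration plus ability and character upgrades.
; On BeginPlay it caches the player's BP_TopDownCharacter, and four trigger boxes respond only when that character overlaps them.
; Two boxes reset current HP or magic to default values.
; The other two open the ability or character upgrade widget and pause the game.
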(event OnComponentBeginOverlap(HealHPTriggerBox)
  (params (OverlappedComponent :type Primitive%20Component%20Object%20Reference) (OtherActor :type Actor%20Object%20Reference) (OtherComp :type Primitive%20Component%20Object%20Reference) (OtherBodyIndex :type Integer) (bFromSweep :type Boolean) (SweepResult :type Hit%20Result%20Structure%20%28by%20ref%29))
  (bind _as_bp_top_down_character (Variables|Default|GetAs%20BP%20Top%20Down%20Character))
  (if (== OtherActor (Variables|Default|GetAs%20BP%20Top%20Down%20Character))
    (Variables|/Game/PlayerCharacter/Blueprints/BP_TopDownCharacter.BP_TopDownCharacter_C|SetCurrentHP _as_bp_top_down_character (Variables|/Game/PlayerCharacter/Blueprints/BP_TopDownCharacter.BP_TopDownCharacter_C|GetDefaultHP _as_bp_top_down_character))))

(event OnComponentBeginOverlap(AbilityUpgradeTriggerBox)
  (params (OverlappedComponent :type Primitive%20Component%20Object%20Reference) (OtherActor :type Actor%20Object%20Reference) (OtherComp :type Primitive%20Component%20Object%20Reference) (OtherBodyIndex :type Integer) (bFromSweep :type Boolean) (SweepResult :type Hit%20Result%20Structure%20%28by%20ref%29))
  (if (== OtherActor (Variables|Default|GetAs%20BP%20Top%20Down%20Character))
    (bind _returnvalue (UserInterface|CreateWidget "/Game/Widget/WB_AbilityUpgrade.WB_AbilityUpgrade_C"))
    (UserInterface|Viewport|AddtoViewport _returnvalue 0)
    (Game|SetGamePaused true)))

(event OnComponentBeginOverlap(CharacterUpgradeTriggerBox)
  (params (OverlappedComponent :type Primitive%20Component%20Object%20Reference) (OtherActor :type Actor%20Object%20Reference) (OtherComp :type Primitive%20Component%20Object%20Reference) (OtherBodyIndex :type Integer) (bFromSweep :type Boolean) (SweepResult :type Hit%20Result%20Structure%20%28by%20ref%29))
  (if (== OtherActor (Variables|Default|GetAs%20BP%20Top%20Down%20Character))
    (bind _returnvalue (UserInterface|CreateWidget "/Game/Widget/WB_CharacterUpgrade.WB_CharacterUpgrade_C"))
    (UserInterface|Viewport|AddtoViewport _returnvalue 0)
    (Game|SetGamePaused true)))

(event OnComponentBeginOverlap(MagicTriggerBox)
  (params (OverlappedComponent :type Primitive%20Component%20Object%20Reference) (OtherActor :type Actor%20Object%20Reference) (OtherComp :type Primitive%20Component%20Object%20Reference) (OtherBodyIndex :type Integer) (bFromSweep :type Boolean) (SweepResult :type Hit%20Result%20Structure%20%28by%20ref%29))
  (bind _as_bp_top_down_character (Variables|Default|GetAs%20BP%20Top%20Down%20Character))
  (if (== OtherActor (Variables|Default|GetAs%20BP%20Top%20Down%20Character))
    (Variables|/Game/PlayerCharacter/Blueprints/BP_TopDownCharacter.BP_TopDownCharacter_C|SetCurrentMagic _as_bp_top_down_character (Variables|/Game/PlayerCharacter/Blueprints/BP_TopDownCharacter.BP_TopDownCharacter_C|GetDefaultMagic _as_bp_top_down_character))))

(event EventBeginPlay
  (|CallParentFunction)
  (bind _asbp_top_down_character (Utilities|Casting|CastToBP_TopDownCharacter (Game|GetPlayerCharacter 0)))
  (Variables|Default|SetAs%20BP%20Top%20Down%20Character _asbp_top_down_character))

(event Collision|EventActorBeginOverlap
  (params (OtherActor :type Actor%20Object%20Reference)))

(event EventTick
  (params (DeltaSeconds :type Float%20%28single-precision%29)))

(fn ConstructionScript
  (|CallParentFunction))