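; BP_RoomParent is a room actor, likely a base for room variants, with four doors that respond to the top-down character.
; Each trigger box plays its door's timeline when the character overlaps it and runs that timeline in reverse from the end on exit.
; Timeline updates add the Open value as a cumulative Z offset to the door rather than setting its position.
; BeginPlay caches the room's XY location in Coordinates.
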(event OnComponentBeginOverlap(Box4)
  (params (OverlappedComponent :type Primitive%20Component%20Object%20Reference) (OtherActor :type Actor%20Object%20Reference) (OtherComp :type Primitive%20Component%20Object%20Reference) (OtherBodyIndex :type Integer) (bFromSweep :type Boolean) (SweepResult :type Hit%20Result%20Structure%20%28by%20ref%29))
  (Utilities|Casting|CastToBP_TopDownCharacter OtherActor)
  (bind _open (Timeline|Timeline Play)
    (:Update
      (Transformation|AddWorldOffset (Variables|Default|GetDoor4) (Math|Vector|MakeVector 0.0 0.0 _open) false false))))

(event OnComponentBeginOverlap(Box3)
  (params (OverlappedComponent :type Primitive%20Component%20Object%20Reference) (OtherActor :type Actor%20Object%20Reference) (OtherComp :type Primitive%20Component%20Object%20Reference) (OtherBodyIndex :type Integer) (bFromSweep :type Boolean) (SweepResult :type Hit%20Result%20Structure%20%28by%20ref%29))
  (Utilities|Casting|CastToBP_TopDownCharacter OtherActor)
  (bind _open (Timeline|Timeline_0 Play)
    (:Update
      (Transformation|AddWorldOffset (Variables|Default|GetDoor3) (Math|Vector|MakeVector 0.0 0.0 _open) false false))))

(event OnComponentBeginOverlap(Box1)
  (params (OverlappedComponent :type Primitive%20Component%20Object%20Reference) (OtherActor :type Actor%20Object%20Reference) (OtherComp :type Primitive%20Component%20Object%20Reference) (OtherBodyIndex :type Integer) (bFromSweep :type Boolean) (SweepResult :type Hit%20Result%20Structure%20%28by%20ref%29))
  (Utilities|Casting|CastToBP_TopDownCharacter OtherActor)
  (bind _open (Timeline|Timeline_1 Play)
    (:Update
      (Transformation|AddWorldOffset (Variables|Default|GetDoor1) (Math|Vector|MakeVector 0.0 0.0 _open) false false))))

(event OnComponentBeginOverlap(Box2)
  (params (OverlappedComponent :type Primitive%20Component%20Object%20Reference) (OtherActor :type Actor%20Object%20Reference) (OtherComp :type Primitive%20Component%20Object%20Reference) (OtherBodyIndex :type Integer) (bFromSweep :type Boolean) (SweepResult :type Hit%20Result%20Structure%20%28by%20ref%29))
  (Utilities|Casting|CastToBP_TopDownCharacter OtherActor)
  (bind _open (Timeline|Timeline_2 Play)
    (:Update
      (Transformation|AddWorldOffset (Variables|Default|GetDoor2) (Math|Vector|MakeVector 0.0 0.0 _open) false false))))

(event OnComponentEndOverlap(Box4)
  (params (OverlappedComponent :type Primitive%20Component%20Object%20Reference) (OtherActor :type Actor%20Object%20Reference) (OtherComp :type Primitive%20Component%20Object%20Reference) (OtherBodyIndex :type Integer))
  (Utilities|Casting|CastToBP_TopDownCharacter OtherActor)
  (bind _open (Timeline|Timeline ReverseFromEnd)
    (:Update
      (Transformation|AddWorldOffset (Variables|Default|GetDoor4) (Math|Vector|MakeVector 0.0 0.0 _open) false false))))

(event OnComponentEndOverlap(Box3)
  (params (OverlappedComponent :type Primitive%20Component%20Object%20Reference) (OtherActor :type Actor%20Object%20Reference) (OtherComp :type Primitive%20Component%20Object%20Reference) (OtherBodyIndex :type Integer))
  (Utilities|Casting|CastToBP_TopDownCharacter OtherActor)
  (bind _open (Timeline|Timeline_0 ReverseFromEnd)
    (:Update
      (Transformation|AddWorldOffset (Variables|Default|GetDoor3) (Math|Vector|MakeVector 0.0 0.0 _open) false false))))

(event OnComponentEndOverlap(Box1)
  (params (OverlappedComponent :type Primitive%20Component%20Object%20Reference) (OtherActor :type Actor%20Object%20Reference) (OtherComp :type Primitive%20Component%20Object%20Reference) (OtherBodyIndex :type Integer))
  (Utilities|Casting|CastToBP_TopDownCharacter OtherActor)
  (bind _open (Timeline|Timeline_1 ReverseFromEnd)
    (:Update
      (Transformation|AddWorldOffset (Variables|Default|GetDoor1) (Math|Vector|MakeVector 0.0 0.0 _open) false false))))

(event OnComponentEndOverlap(Box2)
  (params (OverlappedComponent :type Primitive%20Component%20Object%20Reference) (OtherActor :type Actor%20Object%20Reference) (OtherComp :type Primitive%20Component%20Object%20Reference) (OtherBodyIndex :type Integer))
  (Utilities|Casting|CastToBP_TopDownCharacter OtherActor)
  (bind _open (Timeline|Timeline_2 ReverseFromEnd)
    (:Update
      (Transformation|AddWorldOffset (Variables|Default|GetDoor2) (Math|Vector|MakeVector 0.0 0.0 _open) false false))))

(event EventBeginPlay
  (bind _returnvalue (Transformation|GetActorLocation))
  (Variables|Default|SetCoordinates (Math|Vector2D|MakeVector2D (.x _returnvalue) (.y _returnvalue))))

(fn ConstructionScript)