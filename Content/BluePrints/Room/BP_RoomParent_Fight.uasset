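; Parent Blueprint for dungeon fight rooms that populates the room with enemies when play begins.
; BeginPlay reads per-level Zombie, Magician and Warrior counts from DungeonGameInstance and passes each to its own spawn function.
; Each function counts down in a wired loop, spawning that enemy class at a random XY offset around the room actor's origin, slightly raised and matching its rotation.
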(event EventBeginPlay
  (bind _asdungeon_game_instance (Utilities|Casting|CastToDungeonGameInstance (Game|GetGameInstance)))
  (bind _output_get (Variables|Default|SetZombieAmount (Variables|/Game/DungeonGameInstance.DungeonGameInstance_C|GetLevelZombieAmount _asdungeon_game_instance)))
  (bind _output_get_2 (Variables|Default|SetMagicianAmount (Variables|/Game/DungeonGameInstance.DungeonGameInstance_C|GetLevelMagicianAmount _asdungeon_game_instance)))
  (bind _output_get_3 (Variables|Default|SetKnightAmount (Variables|/Game/DungeonGameInstance.DungeonGameInstance_C|GetLevelWarriorAmount _asdungeon_game_instance)))
  (Utilities|FlowControl|Sequence
    (:then_0
      (CallFunction|SpawnMagician _output_get_2))
    (:then_1
      (CallFunction|SpawnZombie _output_get))
    (:then_2
      (CallFunction|SpawnKnight _output_get_3))))

(fn ConstructionScript)

(fn SpawnZombie
  (params (Amount :type Integer))
  (bind _returnvalue (Transformation|GetActorTransform))
  (if (not (== Amount 0)) :!label _label
    (Game|SpawnActorfromClass "/Game/BluePrints/Enemy/BP_Enemy_Zombie.BP_Enemy_Zombie_C" (Math|Transform|MakeTransform (Math|Vector|MakeVector (+ (Math|Random|RandomFloatinRange -2.5e+02 2.5e+02) (.x (.location _returnvalue))) (+ (.y (.location _returnvalue)) (Math|Random|RandomFloatinRange -2.5e+02 2.5e+02)) (+ (.z (.location _returnvalue)) 5e+01)) (.rotation _returnvalue) "1.000000,1.000000,1.000000") "Undefined" "MultiplyWithRoot" 0 0)
    (Math|Integer|DecrementInt Amount
      (:%20%20
        (goto _label)))))

(fn SpawnMagician
  (params (Amount :type Integer))
  (bind _returnvalue (Transformation|GetActorTransform))
  (if (not (== Amount 0)) :!label _label
    (Game|SpawnActorfromClass "/Game/BluePrints/Enemy/BP_Enemy_Magician.BP_Enemy_Magician_C" (Math|Transform|MakeTransform (Math|Vector|MakeVector (+ (Math|Random|RandomFloatinRange -2.5e+02 2.5e+02) (.x (.location _returnvalue))) (+ (.y (.location _returnvalue)) (Math|Random|RandomFloatinRange -2.5e+02 2.5e+02)) (+ (.z (.location _returnvalue)) 5e+01)) (.rotation _returnvalue) "1.000000,1.000000,1.000000") "Undefined" "MultiplyWithRoot" 0 0)
    (Math|Integer|DecrementInt Amount
      (:%20%20
        (goto _label)))))

(fn SpawnKnight
  (params (Amount :type Integer))
  (bind _returnvalue (Transformation|GetActorTransform))
  (if (not (== Amount 0)) :!label _label
    (Game|SpawnActorfromClass "/Game/BluePrints/Enemy/BP_Enemy_Warrior.BP_Enemy_Warrior_C" (Math|Transform|MakeTransform (Math|Vector|MakeVector (+ (Math|Random|RandomFloatinRange -2.5e+02 2.5e+02) (.x (.location _returnvalue))) (+ (.y (.location _returnvalue)) (Math|Random|RandomFloatinRange -2.5e+02 2.5e+02)) (+ (.z (.location _returnvalue)) 5e+01)) (.rotation _returnvalue) "1.000000,1.000000,1.000000") "Undefined" "MultiplyWithRoot" 0 0)
    (Math|Integer|DecrementInt Amount
      (:%20%20
        (goto _label)))))