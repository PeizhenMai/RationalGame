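; BP_NextLevel is a level-exit trigger actor that sends the player on to the next room in the dungeon sequence.
; On BeginPlay it caches the top-down player character and the DungeonGameInstance.
; When that character overlaps the Box, it takes the entry after the current LevelName in the instance's LevelArray, without a bounds check.
; That entry is the DT_Room row name, and the found row's LevelName is the level it opens.
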(event OnComponentBeginOverlap(Box)
  (params (OverlappedComponent :type Primitive%20Component%20Object%20Reference) (OtherActor :type Actor%20Object%20Reference) (OtherComp :type Primitive%20Component%20Object%20Reference) (OtherBodyIndex :type Integer) (bFromSweep :type Boolean) (SweepResult :type Hit%20Result%20Structure%20%28by%20ref%29))
  (bind _as_dungeon_game_instance (Variables|Default|GetAs%20Dungeon%20Game%20Instance))
  (if (== OtherActor (Variables|Default|GetAs%20BP%20Top%20Down%20Character))
    (bind _returnvalue (Utilities|GetDataTableRow "/Game/DataTable/DT_Room.DT_Room" (Utilities|Array|Get(acopy) (Variables|/Game/DungeonGameInstance.DungeonGameInstance_C|GetLevelArray _as_dungeon_game_instance) (+ 1 (Utilities|Array|FindItem (Variables|/Game/DungeonGameInstance.DungeonGameInstance_C|GetLevelArray _as_dungeon_game_instance) (Variables|/Game/DungeonGameInstance.DungeonGameInstance_C|GetLevelName _as_dungeon_game_instance)))))
      (:then
        (Game|OpenLevel(byName) (.levelname _returnvalue) false)))))

(event EventBeginPlay
  (bind _asbp_top_down_character (Utilities|Casting|CastToBP_TopDownCharacter (Game|GetPlayerCharacter 0)))
  (Variables|Default|SetAs%20BP%20Top%20Down%20Character _asbp_top_down_character)
  (bind _asdungeon_game_instance (Utilities|Casting|CastToDungeonGameInstance (Game|GetGameInstance)))
  (Variables|Default|SetAs%20Dungeon%20Game%20Instance _asdungeon_game_instance))

(event Collision|EventActorBeginOverlap
  (params (OtherActor :type Actor%20Object%20Reference)))

(event EventTick
  (params (DeltaSeconds :type Float%20%28single-precision%29)))

(fn ConstructionScript)