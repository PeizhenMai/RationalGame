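; Dungeon generator actor that builds a random chain of rooms on a grid, using size, scale and count from DungeonGameInstance.
; After BeginPlay, it spawns a start room, fight rooms each paired with an obstacle, then an end room.
; Each step shuffles the previous room's four neighbor cells and checks them against the Rooms map for a free spot.
; Fight rooms link both ways to their predecessor via RoomConnection; the end room is left unlinked.
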(event EventBeginPlay
  (Utilities|FlowControl|Delay 0.2)
  (bind _asdungeon_game_instance (Utilities|Casting|CastToDungeonGameInstance (Game|GetGameInstance)))
  (bind _output_get (Variables|Default|SetRoomSize (Variables|/Game/DungeonGameInstance.DungeonGameInstance_C|GetLevelRoomSize _asdungeon_game_instance)))
  (bind _output_get_2 (Variables|Default|SetRoomScale (Variables|/Game/DungeonGameInstance.DungeonGameInstance_C|GetLevelRoomScale _asdungeon_game_instance)))
  (bind _output_get_3 (Variables|Default|SetRoomAmount (Variables|/Game/DungeonGameInstance.DungeonGameInstance_C|GetLevelRoomAmount _asdungeon_game_instance)))
  (Variables|Default|SetRoomsLeft (Variables|Default|GetRoomAmount))
  (bind _returnvalue (Game|SpawnActorfromClass "/Game/BluePrints/Room/BP_RoomParent_Start.BP_RoomParent_Start_C" (Math|Transform|MakeTransform "0, 0, 0" "0, 0, 0" (Variables|Default|GetRoomScale)) "Undefined" "MultiplyWithRoot" 0 0))
  (bind _output_get_4 (Variables|Default|SetStartRoom _returnvalue))
  (Utilities|Map|Add (Variables|Default|GetRooms) _output_get_4 (Math|Vector2D|MakeVector2D (.x (Transformation|GetActorLocation _returnvalue)) (.y (Transformation|GetActorLocation _returnvalue))))
  (Variables|Default|SetPreviousRoom (Variables|Default|GetStartRoom))
  (bind _result (Math|Integer|DecrementInt (Variables|Default|GetRoomsLeft))
    (:%20%20
      (Variables|Default|SetRoomsLeft _result)
      (if (> (Variables|Default|GetRoomsLeft) 1) :!label _label
        (CallFunction|SpawnRandomRoom)
        (goto _label)
        (else
          (CallFunction|SpawnEndRoom))))))

(event EventTick
  (params (DeltaSeconds :type Float%20%28single-precision%29)))

(fn ConstructionScript)

(fn SpawnRandomRoom
  (bind _roomscale (Variables|Default|GetRoomScale))
  (bind _potentiallocationarray (LocalVariables|GetPotentialLocationArray))
  (Utilities|Array|Add _potentiallocationarray (Math|Vector2D|MakeVector2D (+ (.X (Math|Vector2D|BreakVector2D (.Value (Utilities|Map|Find (Variables|Default|GetRooms) (Variables|Default|GetPreviousRoom))))) (.x (Variables|Default|GetRoomSize))) (.Y (Math|Vector2D|BreakVector2D (.Value (Utilities|Map|Find (Variables|Default|GetRooms) (Variables|Default|GetPreviousRoom)))))))
  (Utilities|Array|Add _potentiallocationarray (Math|Vector2D|MakeVector2D (.X (Math|Vector2D|BreakVector2D (.Value (Utilities|Map|Find (Variables|Default|GetRooms) (Variables|Default|GetPreviousRoom))))) (+ (.Y (Math|Vector2D|BreakVector2D (.Value (Utilities|Map|Find (Variables|Default|GetRooms) (Variables|Default|GetPreviousRoom))))) (.y (Variables|Default|GetRoomSize)))))
  (Utilities|Array|Add _potentiallocationarray (Math|Vector2D|MakeVector2D (- (.X (Math|Vector2D|BreakVector2D (.Value (Utilities|Map|Find (Variables|Default|GetRooms) (Variables|Default|GetPreviousRoom))))) (.x (Variables|Default|GetRoomSize))) (.Y (Math|Vector2D|BreakVector2D (.Value (Utilities|Map|Find (Variables|Default|GetRooms) (Variables|Default|GetPreviousRoom)))))))
  (Utilities|Array|Add _potentiallocationarray (Math|Vector2D|MakeVector2D (.X (Math|Vector2D|BreakVector2D (.Value (Utilities|Map|Find (Variables|Default|GetRooms) (Variables|Default|GetPreviousRoom))))) (- (.Y (Math|Vector2D|BreakVector2D (.Value (Utilities|Map|Find (Variables|Default|GetRooms) (Variables|Default|GetPreviousRoom))))) (.y (Variables|Default|GetRoomSize)))))
  (Utilities|Array|Shuffle _potentiallocationarray)
  (bind _array_element (Utilities|Array|ForEachLoopwithBreak _potentiallocationarray :!label _label)
    (:LoopBody
      (bind _output_get (LocalVariables|SetPotentialLocation _array_element))
      (bind _values (Utilities|Map|Values (Variables|Default|GetRooms)))
      (if (Utilities|Array|ContainsItem _values _output_get)
        (Development|PrintString "HasRoom" true true "(R=0.000000,G=0.660000,B=1.000000,A=1.000000)" 1.0)
        (else
          (goto _label Break))))
    (:Completed
      (Game|SpawnActorfromClass "/Game/BluePrints/BP_Obstacle.BP_Obstacle_C" (Math|Transform|MakeTransform (Math|Vector|MakeVector (.X (Math|Vector2D|BreakVector2D (LocalVariables|GetPotentialLocation))) (.Y (Math|Vector2D|BreakVector2D (LocalVariables|GetPotentialLocation))) 0.0) "0, 0, 0" _roomscale) "Undefined" "MultiplyWithRoot" 0 0)
      (bind _returnvalue (Game|SpawnActorfromClass "/Game/BluePrints/Room/BP_RoomParent_Fight.BP_RoomParent_Fight_C" (Math|Transform|MakeTransform (Math|Vector|MakeVector (.X (Math|Vector2D|BreakVector2D (LocalVariables|GetPotentialLocation))) (.Y (Math|Vector2D|BreakVector2D (LocalVariables|GetPotentialLocation))) 0.0) "0, 0, 0" _roomscale) "Undefined" "MultiplyWithRoot" 0 0))
      (bind _output_get_2 (LocalVariables|SetCurrentRoom _returnvalue))
      (Utilities|Map|Add (Variables|Default|GetRooms) _output_get_2 (Math|Vector2D|MakeVector2D (.x (Transformation|GetActorLocation _returnvalue)) (.y (Transformation|GetActorLocation _returnvalue))))
      (bind _result (Math|Integer|DecrementInt (Variables|Default|GetRoomsLeft))
        (:%20%20
          (Variables|Default|SetRoomsLeft _result)
          (Utilities|Set|Add (Variables|/Game/BluePrints/Room/BP_RoomParent.BP_RoomParent_C|GetRoomConnection (LocalVariables|GetCurrentRoom)) (Variables|Default|GetPreviousRoom))
          (Utilities|Set|Add (Variables|/Game/BluePrints/Room/BP_RoomParent.BP_RoomParent_C|GetRoomConnection (Variables|Default|GetPreviousRoom)) (LocalVariables|GetCurrentRoom))
          (Variables|Default|SetPreviousRoom (LocalVariables|GetCurrentRoom)))))))

(fn SpawnEndRoom
  (bind _rooms (Variables|Default|GetRooms))
  (bind _previousroom (Variables|Default|GetPreviousRoom))
  (bind _potentiallocationarray (LocalVariables|GetPotentialLocationArray))
  (bind _value (Utilities|Map|Find _rooms _previousroom))
  (bind (_x _y) (Math|Vector2D|BreakVector2D _value))
  (bind (_x_2 _y_2) (Math|Vector2D|BreakVector2D _value))
  (bind (_x_3 _y_3) (Math|Vector2D|BreakVector2D _value))
  (bind (_x_4 _y_4) (Math|Vector2D|BreakVector2D _value))
  (Utilities|Array|Add _potentiallocationarray (Math|Vector2D|MakeVector2D (+ _x (.x (Variables|Default|GetRoomSize))) _y))
  (Utilities|Array|Add _potentiallocationarray (Math|Vector2D|MakeVector2D _x_2 (+ _y_2 (.y (Variables|Default|GetRoomSize)))))
  (Utilities|Array|Add _potentiallocationarray (Math|Vector2D|MakeVector2D (- _x_3 (.x (Variables|Default|GetRoomSize))) _y_3))
  (Utilities|Array|Add _potentiallocationarray (Math|Vector2D|MakeVector2D _x_4 (- _y_4 (.y (Variables|Default|GetRoomSize)))))
  (Utilities|Array|Shuffle _potentiallocationarray)
  (bind _array_element (Utilities|Array|ForEachLoopwithBreak _potentiallocationarray :!label _label)
    (:LoopBody
      (bind _output_get (LocalVariables|SetPotentialLocation _array_element))
      (bind _values (Utilities|Map|Values (Variables|Default|GetRooms)))
      (if (Utilities|Array|ContainsItem _values _output_get)
        (Development|PrintString "HasRoom" true true "(R=0.000000,G=0.660000,B=1.000000,A=1.000000)" 1.0)
        (else
          (goto _label Break))))
    (:Completed
      (Game|SpawnActorfromClass "/Game/BluePrints/Room/BP_RoomParent_End.BP_RoomParent_End_C" (Math|Transform|MakeTransform (Math|Vector|MakeVector (.X (Math|Vector2D|BreakVector2D (LocalVariables|GetPotentialLocation))) (.Y (Math|Vector2D|BreakVector2D (LocalVariables|GetPotentialLocation))) 0.0) "0, 0, 0" (Variables|Default|GetRoomScale)) "Undefined" "MultiplyWithRoot" 0 0)
      (bind _result (Math|Integer|DecrementInt (Variables|Default|GetRoomsLeft))
        (:%20%20
          (Variables|Default|SetRoomsLeft _result))))))